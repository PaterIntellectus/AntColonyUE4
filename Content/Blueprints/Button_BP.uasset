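; Button_BP is a floor pressure button that spawns an ant from its linked anthill when something steps on it.
; The first overlap with the collision box sets Pressed, calls SpawnAnt on RelatedAnthill and plays the Push timeline, which moves the button mesh along Z.
; When the last overlapping actor leaves, it clears Pressed and reverses the timeline, re-arming the button for another spawn.
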(event OnComponentBeginOverlap(CollisionBox)
  (params (OverlappedComponent :type Primitive%20Component%20Object%20Reference) (OtherActor :type Actor%20Object%20Reference) (OtherComp :type Primitive%20Component%20Object%20Reference) (OtherBodyIndex :type Integer) (bFromSweep :type Boolean) (SweepResult :type Hit%20Result%20Structure%20%28by%20ref%29))
  (if (not (Variables|Default|GetPressed))
    (Variables|Default|SetPressed true)
    (Default|SpawnAnt (Variables|Default|GetRelatedAnthill))
    (bind _z_location (Timeline|Push Play)
      (:Update
        (Transformation|SetRelativeLocation (Variables|Default|GetButton) (Math|Vector|MakeVector 0.0 0.0 _z_location) false false)))))

(event OnComponentEndOverlap(CollisionBox)
  (params (OverlappedComponent :type Primitive%20Component%20Object%20Reference) (OtherActor :type Actor%20Object%20Reference) (OtherComp :type Primitive%20Component%20Object%20Reference) (OtherBodyIndex :type Integer))
  (if (not (Utilities|Array|IsValidIndex (Collision|GetOverlappingActors (Variables|Default|GetCollisionBox) 0 :!class /Script/Engine.PrimitiveComponent)))
    (Variables|Default|SetPressed false)
    (bind _z_location (Timeline|Push Reverse)
      (:Update
        (Transformation|SetRelativeLocation (Variables|Default|GetButton) (Math|Vector|MakeVector 0.0 0.0 _z_location) false false)))))

(event EventBeginPlay)

(event Collision|EventActorBeginOverlap
  (params (OtherActor :type Actor%20Object%20Reference)))

(event EventTick
  (params (DeltaSeconds :type Float%20%28single-precision%29)))

(fn ConstructionScript)