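; AI ant pawn that travels to a target actor, then plays an insect digging sound and destroys itself on arrival.
; BeginMoveToTarget stores the target, home and phase timings, moving straight to the target when all timings are zero.
; Otherwise it loops through timed phases of advancing, pausing and retreating home, skipping zero-length ones.
; Delays run alongside AIMoveTo, and each new move or stop cuts the current one short.
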(event Custom|BeginMoveToTarget
  (params (Target%20Actor :type Target%20Point%20Object%20Reference) (Home :type Anthill%20BP%20Object%20Reference) (MoveToTargetTime :type Float%20%28single-precision%29) (StopMoveTime :type Float%20%28single-precision%29) (MoveHomeTime :type Float%20%28single-precision%29))
  (CallFunction|SetMoveSettings Target%20Actor Home MoveToTargetTime StopMoveTime MoveHomeTime)
  (if (Math|Boolean|ANDBoolean (== (Variables|Default|GetMoveToTargetTime) 0.0) (== (Variables|Default|GetStopMoveTime) 0.0) (== (Variables|Default|GetMoveHomeTime) 0.0))
    (AI|AIMoveTo self "0, 0, 0" (Variables|Default|GetTarget%20Point) 5.0 false
      (:OnSuccess
        _))
    (else
      (AI|AIMoveTo self "0, 0, 0" (Variables|Default|GetTarget%20Point) 5.0 false :!label _label
        (:then
          (if (!= (Variables|Default|GetMoveToTargetTime) 0.0)
            (Utilities|FlowControl|Delay (Variables|Default|GetMoveToTargetTime)))
          (if (!= (Variables|Default|GetStopMoveTime) 0.0)
            (Class|NavMovementComponent|StopActiveMovement (Variables|Character|GetCharacterMovement))
            (Utilities|FlowControl|Delay (Variables|Default|GetStopMoveTime)))
          (if (!= (Variables|Default|GetMoveHomeTime) 0.0)
            (AI|AIMoveTo self "0, 0, 0" (Variables|Default|GetHome) 5.0 false
              (:then
                (Utilities|FlowControl|Delay (Variables|Default|GetMoveHomeTime))
                (goto _label)))
            (else
              (goto _label))))
        (:OnSuccess
          _))))
  (Audio|PlaySoundatLocation "/Game/Sounds/ES_InsectDigFoliage_SFX.ES_InsectDigFoliage_SFX" (Transformation|GetActorLocation) "0, 0, 0" 1.0 1.0 0.0 0 0 0)
  (Actor|DestroyActor))

(fn ConstructionScript)

(fn SetMoveSettings
  (params (Target%20Point :type Target%20Point%20Object%20Reference) (Home :type Anthill%20BP%20Object%20Reference) (MoveToTargetTime :type Float%20%28single-precision%29) (StopMoveTime :type Float%20%28single-precision%29) (MoveToHomeTime :type Float%20%28single-precision%29))
  (Variables|Default|SetTarget%20Point Target%20Point)
  (Variables|Default|SetHome Home)
  (Variables|Default|SetMoveToTargetTime MoveToTargetTime)
  (Variables|Default|SetStopMoveTime StopMoveTime)
  (Variables|Default|SetMoveHomeTime MoveToHomeTime))