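; Anthill actor that spawns an AI ant and sends it out toward a target point, with itself as the ant's home.
; SpawnAnt runs only when the last spawned ant is no longer valid, so each hill keeps one ant at a time.
; It plays a digging sound, spawns the ant at the hill and passes it the move-out, stop and return timings.
; The event graph is empty, so SpawnAnt relies on an outside caller.
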(event EventBeginPlay)

(event Collision|EventActorBeginOverlap
  (params (OtherActor :type Actor%20Object%20Reference)))

(event EventTick
  (params (DeltaSeconds :type Float%20%28single-precision%29)))

(fn ConstructionScript)

(fn SpawnAnt
  (bind _returnvalue (Transformation|GetActorLocation))
  (Utilities|IsValid (Variables|Default|GetLast%20Ant)
    (:Is%20Not%20Valid
      (Audio|PlaySoundatLocation "/Game/Sounds/ES_InsectDigDirt_SFX.ES_InsectDigDirt_SFX" _returnvalue "0, 0, 0" 1.0 1.0 0.0 0 0 0)
      (bind _returnvalue_2 (AI|SpawnAIFromClass "/Game/Blueprints/Ant/AIBP_Ant.AIBP_Ant_C" 0 _returnvalue "0, 0, 0" false 0))
      (bind _asaibp_ant (Utilities|Casting|CastToAIBP_Ant _returnvalue_2))
      (bind _output_get (Variables|Default|SetLast%20Ant _asaibp_ant))
      (Default|BeginMovetoTarget _output_get (Variables|Default|GetTarget%20Point) self (Variables|Default|GetAntsMoveToTargetTime) (Variables|Default|GetAntsStopMoveTime) (Variables|Default|GetAntsMoveToHomeTime)))))